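; Player character Blueprint that handles automatic rifle fire while the Fire input is held.
; A looping timer repeats AutomaticFire, which plays shot sound and muzzle flash, spawns a tracer actor and decrements ammo.
; CalculateShootInfo traces from the camera and aims the tracer from the muzzle socket at the hit point or trace end.
; Ammo never gates firing here, as CanShoot is only set true.
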(event Custom|AutomaticFire
  (if (Variables|Default|GetFiring)
    (if (Variables|Default|GetbCanShoot)
      (Audio|PlaySoundatLocation "/Game/Sound/Weapons/SMG_Thompson/Cue_Thompson_Shot.Cue_Thompson_Shot" (Transformation|GetActorLocation (Game|Player|GetPlayerPawn 0)))
      (Effects|SpawnEmitteratLocation "/Game/Effects/P_AssaultRifle_MF.P_AssaultRifle_MF" (Transformation|GetSocketLocation (Variables|Default|GetGun) "MuzzleFlashSocket") "0.000000,90.000000,0.000000")
      (bind _shoottolocation (CallFunction|CalculateShootInfo))
      (Game|SpawnActorfromClass "/Game/Weapons/RifleTracer_BP.RifleTracer_BP_C" _shoottolocation "Undefined" 0 0)
      (Variables|Default|Setammo (- (Variables|Default|Getammo) 1)))))

(event EventBeginPlay
  (Variables|Default|SetPlayerCamera (Variables|Default|GetFollowCamera))
  (Variables|Default|Setammo (Variables|Default|GetmaxAmmo))
  (Variables|Default|SetbCanShoot true))

(event Input|ActionEvents|InputActionFire
  (params (Key :type Key%20Structure :default "AnyKey"))
  (:Pressed
    (Variables|Default|SetFiring true)
    (CallFunction|AutomaticFire)
    (bind _returnvalue (Utilities|Time|SetTimerbyEvent (delegate Custom|AutomaticFire) (Variables|Default|GetfiringRate) true))
    (Variables|Default|SetTimer _returnvalue))
  (:Released
    (Variables|Default|SetFiring false)
    (Utilities|Time|ClearandInvalidateTimerbyHandle (Variables|Default|GetTimer))))

(fn ConstructionScript)

(fn CalculateShootInfo
  (bind _playercamera (Variables|Default|GetPlayerCamera))
  (bind _gun (Variables|Default|GetGun))
  (bind _returnvalue (Transformation|GetWorldLocation _playercamera))
  (bind _returnvalue_2 (Math|Vector|GetForwardVector _playercamera))
  (bind _returnvalue_3 (Transformation|GetSocketLocation _gun "MuzzleFlashSocket"))
  (bind _returnvalue_4 (* _returnvalue_2 1e+04))
  (bind _returnvalue_5 (+ _returnvalue _returnvalue_4))
  (bind (_outhit _returnvalue_6) (Collision|LineTraceByChannel _returnvalue _returnvalue_5 "TraceTypeQuery1" false 0 "None"))
  (if _returnvalue_6
    (return (Math|Transform|MakeTransform _returnvalue_3 (Math|Rotator|FindLookatRotation _returnvalue_3 (.ImpactPoint (Collision|BreakHitResult _outhit)))))
    (else
      (return (Math|Transform|MakeTransform _returnvalue_3 (Math|Rotator|FindLookatRotation _returnvalue_3 _returnvalue_5))))))